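; Player hero character for a twin-stick shooter, handling movement, aiming, shooting and death.
; BeginPlay spawns a weapon attached to GunTemp and stores the hero's start transform in the TwinStickGameMode as the respawn point.
; Move axes drive world-space movement, while look axes share logic that sets control rotation and holds the trigger during non-zero input.
; AffectHealth applies damage and, on death, requests a respawn before destroying weapon and hero.
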(event EventBeginPlay
  (bind _guntemp (Variables|Default|GetGunTemp))
  (Utilities|FlowControl|Sequence
    (:then_0
      ;[1 1 1] weapon setup
      (bind _returnvalue (Game|SpawnActorfromClass "/Game/Blueprints/Weapon.Weapon_C" (Transformation|GetWorldTransform _guntemp) "Undefined" 0 0))
      (bind _output_get (Variables|Default|SetWeapon _returnvalue))
      (Transformation|AttachComponentToComponent _output_get _guntemp "None" "SnapToTarget" "KeepRelative" "KeepWorld" true))
    (:then_1
      ;[1 1 1] game mode respawn
      (bind _astwin_stick_game_mode (Utilities|Casting|CastToTwinStickGameMode (Game|GetGameMode)))
      (bind _output_get_2 (Variables|Default|SetGameMode _astwin_stick_game_mode))
      (Variables|/Game/Blueprints/TwinStickGameMode.TwinStickGameMode_C|SetSpawnTransform _output_get_2 (Transformation|GetActorTransform)))))

(event Collision|EventActorBeginOverlap
  (params (OtherActor :type Actor%20Object%20Reference)))

(event EventTick
  (params (DeltaSeconds :type Float%20%28single-precision%29)))

(event EventAffectHealth
  (params (Delta :type Float%20%28single-precision%29))
  ;[1 1 1] damage player
  (Class|BaseCharacter|CalculateHealth Delta)
  (if (Variables|Default|GetisDead)
    (Default|RespawnPlayer (Variables|Default|GetGameMode))
    (Actor|DestroyActor (Variables|Default|GetWeapon))))

(event Input|AxisEvents|InputAxisMoveUp
  (params (AxisValue :type Float%20%28single-precision%29))
  ;[1 1 1] Movement
  (Pawn|Input|AddMovementInput "1.000000, 0, 0" AxisValue false))

(event Input|AxisEvents|InputAxisLookRight
  (params (AxisValue :type Float%20%28single-precision%29))
  (bind _weapon (Variables|Default|GetWeapon))
  ;[1 1 1] rotation
  (if (> (Math|Vector|VectorLength (Math|Vector|MakeVector (stale Input|AxisEvents|InputAxisLookUp AxisValue) AxisValue 0.0)) 0.0)
    (Pawn|SetControlRotation (Pawn|GetController) (Math|Conversions|RotationFromXVector (Math|Vector|MakeVector (stale Input|AxisEvents|InputAxisLookUp AxisValue) AxisValue 0.0)))
    (Default|PullTrigger _weapon)
    (else
      (Default|ReleaseTrigger _weapon))))

(event Input|AxisEvents|InputAxisLookUp
  (params (AxisValue :type Float%20%28single-precision%29))
  (bind _weapon (Variables|Default|GetWeapon))
  ;[1 1 1] rotation
  (if (> (Math|Vector|VectorLength (Math|Vector|MakeVector AxisValue (stale Input|AxisEvents|InputAxisLookRight AxisValue) 0.0)) 0.0)
    (Pawn|SetControlRotation (Pawn|GetController) (Math|Conversions|RotationFromXVector (Math|Vector|MakeVector AxisValue (stale Input|AxisEvents|InputAxisLookRight AxisValue) 0.0)))
    (Default|PullTrigger _weapon)
    (else
      (Default|ReleaseTrigger _weapon))))

(event Input|AxisEvents|InputAxisMoveRight
  (params (AxisValue :type Float%20%28single-precision%29))
  ;[1 1 1] Movement
  (Pawn|Input|AddMovementInput "0.000000,1.000000, 0" AxisValue false))

(fn ConstructionScript)